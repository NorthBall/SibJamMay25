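; Player controller that adds the input mapping context and runs the game's UI, music and story flow from prologue to epilogue.
; Creates the HUD, menu and death widgets hidden, and builds audio components for menu music and a random-track pool.
; Story events show numbered slide widgets with voiceover, revealing cursor and Next button after delays.
; The Story value selects each slide, starts gameplay after the prologue, and ends the epilogue with a quit widget.
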(event `StartGame`
  (set `self.Game Start` true)
  (bind _asgame_instans_play (cast `/Game/BP/GameInstans_Play` (`GameplayStatics.GetGameInstance`)))
  (set `self.As Game Instans Play` _asgame_instans_play)
  (`self.Music Meneger`)
  (`Widget.SetVisibility` (`self.Ref W HUD`) "Visible")
  (`Widget.SetVisibility` (`self.Ref Menu Play`) "Hidden")
  (`Widget.SetVisibility` (`self.Ref W YouDead`) "Hidden")
  (`WidgetBlueprintLibrary.SetInputMode_GameAndUIEx` (`GameplayStatics.GetPlayerController` 0) null)
  (`GameplayStatics.PlaySound2D` null (`/Game/BP/GameInstans_Play.Music_Volume_GI` (`self.As Game Instans Play`)) 1.0 0.0 null null)
  (bind _returnvalue (`|CreateWidget` "/Game/UI/HUD/W_Support.W_Support_C"))
  (`UserWidget.AddToViewport` _returnvalue 0))

(event `self.ReceiveBeginPlay`
  (`EnhancedInputSubsystemInterface.AddMappingContext` (subsystem `EnhancedInputLocalPlayerSubsystem`) "/Game/Player/Input/IMC_Main.IMC_Main" 0 (struct)))

(event `self.ReceiveTick`
  (params (DeltaSeconds :type "Float (single-precision)")))

(event `Visibility HUD`
  ;[1 1 1] Создание HUD
  (bind _returnvalue (`|CreateWidget` "/Game/UI/HUD/W_HUD.W_HUD_C"))
  (bind _output_get (set `self.Ref W HUD` _returnvalue))
  (`UserWidget.AddToViewport` _output_get 0)
  (`Widget.SetVisibility` _output_get "Hidden")
  (bind _returnvalue_2 (`|CreateWidget` "/Game/UI/Menu/W_MenuPlay.W_MenuPlay_C" null null null))
  (bind _output_get_2 (set `self.Ref Menu Play` _returnvalue_2))
  (`Widget.SetVisibility` _output_get_2 "Hidden")
  (`UserWidget.AddToViewport` _output_get_2 0)
  (bind _returnvalue_3 (`|CreateWidget` "/Game/UI/HUD/W_YouDead.W_YouDead_C"))
  (bind _output_get_3 (set `self.Ref W YouDead` _returnvalue_3))
  (`Widget.SetVisibility` _output_get_3 "Hidden")
  (`UserWidget.AddToViewport` _output_get_3 0))

(event `Music Meneger`
  ;[1 0.7783 0.05708 0.5] Менеджер музыки (Нужно добавить музыку)
  (`|ExecutionSequence`
    (:`then_0`
      (bind _returnvalue (`AddComponent|NODE_AddAudioComponent-5`))
      (bind _output_get (set `self.Ref Music Menu` _returnvalue))
      (`AudioComponent.Stop` _output_get))
    (:`then_1`
      (bind _returnvalue_2 (`AddComponent|NODE_AddAudioComponent-6`))
      (`AudioComponent.Stop` _returnvalue_2)
      (`KismetArrayLibrary.Array_Add` (`self.All_Array_Music_Normal`) _returnvalue_2))
    (:`then_2`
      (bind _returnvalue_3 (`AddComponent|NODE_AddAudioComponent-7`))
      (`AudioComponent.Stop` _returnvalue_3)
      (`KismetArrayLibrary.Array_Add` (`self.All_Array_Music_Normal`) _returnvalue_3))
    (:`then_3`
      (bind _returnvalue_4 (`AddComponent|NODE_AddAudioComponent-8`))
      (`AudioComponent.Stop` _returnvalue_4)
      (`KismetArrayLibrary.Array_Add` (`self.All_Array_Music_Normal`) _returnvalue_4))
    (:`then_4`
      (bind _returnvalue_5 (`AddComponent|NODE_AddAudioComponent-9`))
      (`AudioComponent.Stop` _returnvalue_5)
      (`KismetArrayLibrary.Array_Add` (`self.All_Array_Music_Normal`) _returnvalue_5))))

(event `Random Music`
  ;[1 0.7783 0.05708 0.5] Менеджер музыки (Нужно добавить музыку)
  (bind _output_get (set `self.Play Music Normal` (`KismetArrayLibrary.Array_Random` (`self.All_Array_Music_Normal`))))
  (`AudioComponent.Play` _output_get 0.0))

(event `Start_Story`
  (bind _returnvalue (`GameplayStatics.GetPlayerController` 0))
  (bind _play_music_normal (`self.Play Music Normal`))
  (`/Engine/EditorBlueprintResources/StandardMacros.IsValid` (`self.As Game Instans Play`)
    (:`Is Valid`
      _)
    (:`Is Not Valid`
      (bind _asgame_instans_play (cast `/Game/BP/GameInstans_Play` (`GameplayStatics.GetGameInstance`)))
      (set `self.As Game Instans Play` _asgame_instans_play)))
  (`self.Music Meneger`)
  (`/Engine/EditorBlueprintResources/StandardMacros.IsValid` _play_music_normal
    (:`Is Valid`
      (`AudioComponent.Stop` _play_music_normal))
    (:`Is Not Valid`
      _))
  (`AudioComponent.Stop` (`self.Ref Music Menu`))
  (`GameplayStatics.PlaySound2D` null (`/Game/BP/GameInstans_Play.Music_Volume_GI` (`self.As Game Instans Play`)) 1.0 0.0 null null) ; МЕЛОДИЯ ПОД ИСТОРИЮ
  (`GameplayStatics.PlaySound2D` null (`/Game/BP/GameInstans_Play.Voice_Volume_GI` (`self.As Game Instans Play`)) 1.0 0.0 null null)
  (bind _returnvalue_2 (`|CreateWidget` "/Game/UI/HUD/W_Next.W_Next_C"))
  (bind _output_get (set `self.Ref W Next` _returnvalue_2))
  (`Widget.SetVisibility` _output_get "Hidden")
  (`UserWidget.AddToViewport` _output_get 1)
  (set `PlayerController.bShowMouseCursor` false _returnvalue)
  (bind _returnvalue_3 (`|CreateWidget` "/Game/UI/Story/Prolog/W_Story_1.W_Story_1_C" _returnvalue))
  (bind _output_get_2 (set `self.Ref Prolog 1` _returnvalue_3))
  (`UserWidget.AddToViewport` _output_get_2 0)
  (`KismetSystemLibrary.Delay` 3.0)
  (set `PlayerController.bShowMouseCursor` true (`GameplayStatics.GetPlayerController` 0))
  (`Widget.SetVisibility` (`self.Ref W Next`) "Visible"))

(event `Next_Story`
  (bind _returnvalue (`GameplayStatics.GetPlayerController` 0))
  (bind _play_music_normal (`self.Play Music Normal`))
  (bind _voice_volume_gi (`/Game/BP/GameInstans_Play.Voice_Volume_GI` (`self.As Game Instans Play`)))
  (bind _voice_volume_gi_2 (`/Game/BP/GameInstans_Play.Voice_Volume_GI` (`self.As Game Instans Play`)))
  (`/Engine/EditorBlueprintResources/StandardMacros.IsValid` (`self.Ref W Next`)
    (:`Is Valid`
      (`Widget.SetVisibility` (`self.Ref W Next`) "Hidden"))
    (:`Is Not Valid`
      ;[1 0.8473 0.1357] Для тестов Епилога
      (bind _returnvalue_2 (`|CreateWidget` "/Game/UI/HUD/W_Next.W_Next_C"))
      (bind _output_get (set `self.Ref W Next` _returnvalue_2))
      (`Widget.SetVisibility` _output_get "Hidden")
      (`UserWidget.AddToViewport` _output_get 1)))
  (`/Engine/EditorBlueprintResources/StandardMacros.IsValid` _play_music_normal
    (:`Is Valid`
      (`AudioComponent.Stop` _play_music_normal))
    (:`Is Not Valid`
      _))
  (`AudioComponent.Stop` (`self.Ref Music Menu`))
  (set `PlayerController.bShowMouseCursor` false _returnvalue)
  (switch `int` (`KismetMathLibrary.FTrunc` (`self.Story`))
    (:`1`
      (`GameplayStatics.PlaySound2D` null _voice_volume_gi 1.0 0.0 null null)
      (bind _returnvalue_3 (`|CreateWidget` "/Game/UI/Story/Prolog/W_Story_2.W_Story_2_C" _returnvalue))
      (bind _output_get_2 (set `self.Ref Prolog 2` _returnvalue_3))
      (`UserWidget.AddToViewport` _output_get_2 0)
      (`KismetSystemLibrary.Delay` 3.0)
      (set `PlayerController.bShowMouseCursor` true (`GameplayStatics.GetPlayerController` 0) :!label _label)
      (`Widget.SetVisibility` (`self.Ref W Next`) "Visible"))
    (:`2`
      (`GameplayStatics.PlaySound2D` null _voice_volume_gi 1.0 0.0 null null)
      (bind _returnvalue_4 (`|CreateWidget` "/Game/UI/Story/Prolog/W_Story_3.W_Story_3_C" _returnvalue))
      (bind _output_get_3 (set `self.Ref Prolog 3` _returnvalue_4))
      (`UserWidget.AddToViewport` _output_get_3 0)
      (`KismetSystemLibrary.Delay` 3.0)
      (goto _label))
    (:`3`
      (`GameplayStatics.PlaySound2D` null _voice_volume_gi 1.0 0.0 null null)
      (bind _returnvalue_5 (`|CreateWidget` "/Game/UI/Story/Prolog/W_Story_4.W_Story_4_C" _returnvalue))
      (bind _output_get_4 (set `self.Ref Prolog 4` _returnvalue_5))
      (`UserWidget.AddToViewport` _output_get_4 0)
      (`KismetSystemLibrary.Delay` 3.0)
      (goto _label))
    (:`4`
      (`Widget.RemoveFromParent` (`self.Ref Prolog 1`))
      (`Widget.RemoveFromParent` (`self.Ref Prolog 2`))
      (`Widget.RemoveFromParent` (`self.Ref Prolog 3`))
      (`Widget.RemoveFromParent` (`self.Ref Prolog 4`))
      (`self.StartGame`))
    (:`5`
      (`GameplayStatics.PlaySound2D` null _voice_volume_gi_2 1.0 0.0 null null)
      (bind _returnvalue_6 (`|CreateWidget` "/Game/UI/Story/Epilog/W_Story_5.W_Story_5_C"))
      (bind _output_get_5 (set `self.Ref Epilog 1` _returnvalue_6))
      (`UserWidget.AddToViewport` _output_get_5 0)
      (`KismetSystemLibrary.Delay` 3.0)
      (set `PlayerController.bShowMouseCursor` true (`GameplayStatics.GetPlayerController` 0) :!label _label_2)
      (`Widget.SetVisibility` (`self.Ref W Next`) "Visible"))
    (:`6`
      (`GameplayStatics.PlaySound2D` null _voice_volume_gi_2 1.0 0.0 null null)
      (bind _returnvalue_7 (`|CreateWidget` "/Game/UI/Story/Epilog/W_Story_6.W_Story_6_C"))
      (bind _output_get_6 (set `self.Ref Epilog 2` _returnvalue_7))
      (`UserWidget.AddToViewport` _output_get_6 0)
      (`KismetSystemLibrary.Delay` 5.0)
      (goto _label_2))
    (:`7`
      (`GameplayStatics.PlaySound2D` null _voice_volume_gi_2 1.0 0.0 null null)
      (bind _returnvalue_8 (`|CreateWidget` "/Game/UI/Story/Epilog/W_Story_7.W_Story_7_C"))
      (bind _output_get_7 (set `self.Ref Epilog 3` _returnvalue_8))
      (`UserWidget.AddToViewport` _output_get_7 0)
      (`KismetSystemLibrary.Delay` 6.0)
      (goto _label_2))
    (:`8`
      (`GameplayStatics.PlaySound2D` null _voice_volume_gi_2 1.0 0.0 null null)
      (bind _returnvalue_9 (`|CreateWidget` "/Game/UI/Story/Epilog/W_Story_8.W_Story_8_C"))
      (bind _output_get_8 (set `self.Ref Epilog 4` _returnvalue_9))
      (`UserWidget.AddToViewport` _output_get_8 0)
      (`KismetSystemLibrary.Delay` 5.0)
      (set `PlayerController.bShowMouseCursor` true (`GameplayStatics.GetPlayerController` 0))
      (bind _returnvalue_10 (`|CreateWidget` "/Game/UI/HUD/W_QuitGame.W_QuitGame_C"))
      (`UserWidget.AddToViewport` _returnvalue_10 1))))

(fn `UserConstructionScript`)