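; Base weapon Blueprint for the player, providing shared ammo, cooldown and reload logic.
; Ammo starts at clip size; timers drive the attack cooldown and reload, which refills the clip when it ends.
; CanAttack is true only while neither timer is active, and CheckAmmo starts a reload when ammo runs out.
; PerformAttack is an empty event, and nothing in this class decrements ammo or calls the cooldown.
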(event `self.ReceiveBeginPlay`
  (set `self.CurrentAmmo` (`self.ClipSize`)))

(event `PerformAttack`)

(event `StartCooldown`
  (bind _returnvalue (`KismetSystemLibrary.K2_SetTimerDelegate` (delegate `ClearCooldown`) (`self.DefaultCooldown`)))
  (set `self.CooldownHandle` _returnvalue))

(event `ClearCooldown`)

(event `StartReload`
  (if (not (`self.IsReloading`))
    (bind _returnvalue (`KismetSystemLibrary.K2_SetTimerDelegate` (delegate `EndReload`) (`self.ReloadTime`)))
    (set `self.ReloadHandle` _returnvalue)))

(event `EndReload`
  (set `self.CurrentAmmo` (`self.ClipSize`)))

(event `CheckAmmo`
  (if (<= (`self.CurrentAmmo`) 0)
    (`self.StartReload`)))

(fn `CanAttack`
  (returns (Result :type Boolean))
  (return (and (not (`KismetSystemLibrary.K2_IsTimerActiveHandle` (`self.CooldownHandle`))) (not (`self.IsReloading`)))))

(fn `IsReloading`
  (returns (IsReloading :type Boolean))
  (return (`KismetSystemLibrary.K2_IsTimerActiveHandle` (`self.ReloadHandle`))))

(fn `UserConstructionScript`)