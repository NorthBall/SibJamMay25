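; Base projectile Blueprint that filters overlaps and provides a damage helper for derived projectiles.
; On overlap it ignores its owner, forwards players and enemies only when AttackPlayer or AttackEnemies allows it, and forwards any other actor unconditionally.
; OnOverlap is an empty event, presumably for children to override.
; DealDamage passes Damage to the target's HealthComponent if one exists.
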(event `self.ReceiveActorBeginOverlap`
  (params (OtherActor :type "Actor Object Reference"))
  (bind _returnvalue (`GameplayStatics.GetObjectClass` OtherActor))
  (if (!= OtherActor (`self.GetOwner`))
    (if (`KismetMathLibrary.ClassIsChildOf` _returnvalue "/Game/Player/BP_PlayerChar.BP_PlayerChar_C")
      (if (`self.AttackPlayer`)
        (`self.OnOverlap` OtherActor))
      (elif (`KismetMathLibrary.ClassIsChildOf` _returnvalue "/Game/Enemies/BP_EnemyBase.BP_EnemyBase_C")
        (if (`self.AttackEnemies`)
          (`self.OnOverlap` OtherActor))
        (else
          (`self.OnOverlap` OtherActor))))))

(event `OnOverlap`
  (params (OtherActor :type "Actor Object Reference")))

(event `DealDamage`
  (params (DamageTarget :type "Actor Object Reference"))
  (bind _returnvalue (`self.GetComponentByClass` DamageTarget "/Game/Player/HealthComponent.HealthComponent_C"))
  (`/Engine/EditorBlueprintResources/StandardMacros.IsValid` _returnvalue
    (:`Is Valid`
      (`/Game/Player/HealthComponent.DealDamage` _returnvalue (`self.Damage`)))))

(fn `UserConstructionScript`)