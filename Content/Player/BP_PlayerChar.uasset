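; Player character Blueprint that handles Enhanced Input movement, look and jump, plus main and alternate attacks through two weapon slots.
; BeginPlay adds Honey and WolfClaws items to per-slot arrays, and an empty slot immediately spawns the item's weapon actor and attaches it to that slot's point.
; Attack inputs call PerformAttack on the slot's current weapon.
; A CanJump flag gates jumping, and Tick prints velocity magnitude for debugging.
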(event `self.ReceiveBeginPlay`
  (bind _returnvalue (`|GenericCreateObject` "/Game/Player/Items/Item_W_Honey.Item_W_Honey_C"))
  (`self.AddNewWeapon` _returnvalue)
  (bind _returnvalue_2 (`|GenericCreateObject` "/Game/Player/Items/Item_W_WolfClaws.Item_W_WolfClaws_C"))
  (`self.AddNewWeapon` _returnvalue_2 true))

(event `self.ReceiveTick`
  (params (DeltaSeconds :type "Float (single-precision)"))
  (`KismetSystemLibrary.PrintString` (`KismetStringLibrary.Conv_DoubleToString` (`KismetMathLibrary.VSize` (`self.GetVelocity`))) true false (struct :`G` 1.0 :`B` 0.212814 :`A` 1.0) 0.0))

(event `EnhancedInput|/Game/Player/Input/IA_Forward`
  (params (ActionValue :type "Vector2D Structure") (ElapsedSeconds :type "Float (double-precision)") (TriggeredSeconds :type "Float (double-precision)") (InputAction :type "InputAction Object Reference" :default "/Game/Player/Input/IA_Forward.IA_Forward"))
  (:`Triggered`
    (`self.AddMovementInput` (`KismetMathLibrary.GreaterGreater_VectorRotator` (`KismetMathLibrary.Conv_Vector2DToVector` ActionValue) (`self.K2_GetActorRotation`)))))

(event `EnhancedInput|/Game/Player/Input/IA_Look`
  (params (ActionValue :type "Vector2D Structure") (ElapsedSeconds :type "Float (double-precision)") (TriggeredSeconds :type "Float (double-precision)") (InputAction :type "InputAction Object Reference" :default "/Game/Player/Input/IA_Look.IA_Look"))
  (:`Triggered`
    (`self.AddControllerYawInput` ActionValue_X)
    (`self.AddControllerPitchInput` ActionValue_Y)))

(event `EnhancedInput|/Game/Player/Input/IA_Jump`
  (params (ActionValue :type Boolean) (ElapsedSeconds :type "Float (double-precision)") (TriggeredSeconds :type "Float (double-precision)") (InputAction :type "InputAction Object Reference" :default "/Game/Player/Input/IA_Jump.IA_Jump"))
  (:`Triggered`
    (`self.Jump`)))

(event `EnhancedInput|/Game/Player/Input/IA_MainAttack`
  (params (ActionValue :type Boolean) (ElapsedSeconds :type "Float (double-precision)") (TriggeredSeconds :type "Float (double-precision)") (InputAction :type "InputAction Object Reference" :default "/Game/Player/Input/IA_MainAttack.IA_MainAttack"))
  (:`Triggered`
    (`self.Attack`)))

(event `EnhancedInput|/Game/Player/Input/IA_AlternateAttack`
  (params (ActionValue :type Boolean) (ElapsedSeconds :type "Float (double-precision)") (TriggeredSeconds :type "Float (double-precision)") (InputAction :type "InputAction Object Reference" :default "/Game/Player/Input/IA_AlternateAttack.IA_AlternateAttack"))
  (:`Triggered`
    (`self.AlternateAttack`)))

(event `AddNewWeapon`
  (params (NewWeapon :type "/Game/Player/Items/BP_Item_Weapon Object Reference") (IsAlternative :type Boolean))
  (`KismetArrayLibrary.Array_AddUnique` (`self.GetWeaponsArray` IsAlternative) NewWeapon)
  (`/Engine/EditorBlueprintResources/StandardMacros.IsValid` (`self.GetCurrentWeapon` IsAlternative)
    (:`Is Not Valid`
      (`self.SetWeapon` NewWeapon IsAlternative))))

(event `SetWeapon`
  (params (NewWeapon :type "/Game/Player/Items/BP_Item_Weapon Object Reference") (IsAlternative :type Boolean))
  (`self.RemoveCurrentWeapon` IsAlternative)
  (bind _returnvalue (`|SpawnActorFromClass` (`/Game/Player/Items/BP_Item_Weapon.WeaponClass` NewWeapon) (`SceneComponent.K2_GetComponentToWorld` (`self.MainWeaponPoint`)) "AlwaysSpawn" "MultiplyWithRoot" self null))
  (`self.K2_AttachToComponent` _returnvalue (`self.GetWeaponPoint` IsAlternative) "None" "SnapToTarget" "SnapToTarget" "SnapToTarget" true)
  (if IsAlternative
    (set `self.CurrentAltWeapon` _returnvalue)
    (else
      (set `self.CurrentMainWeapon` _returnvalue))))

(event `RemoveCurrentWeapon`
  (params (IsAlternative :type Boolean))
  (if IsAlternative
    (bind _currentaltweapon (`self.CurrentAltWeapon`)
      (:`then`
        (`self.K2_DestroyActor` _currentaltweapon))
      (:`else`))
    (else
      (bind _currentmainweapon (`self.CurrentMainWeapon`)
        (:`then`
          (`self.K2_DestroyActor` _currentmainweapon))
        (:`else`)))))

(event `Attack`
  (bind _currentmainweapon (`self.CurrentMainWeapon`)
    (:`then`
      (`/Game/Player/Weapon/BP_Weapon_Base.PerformAttack` _currentmainweapon))
    (:`else`)))

(event `AlternateAttack`
  (bind _currentaltweapon (`self.CurrentAltWeapon`)
    (:`then`
      (`/Game/Player/Weapon/BP_Weapon_Base.PerformAttack` _currentaltweapon))
    (:`else`)))

(fn `CanJumpInternal`
  (returns (ReturnValue :type Boolean))
  (if (`self.bCanJump`)
    (bind _returnvalue (`parent.CanJumpInternal`))
    (return _returnvalue)
    (else
      (return false))))

(fn `GetCurrentWeapon`
  (params (IsAlternative :type Boolean))
  (returns (CurrentWeapon :type "/Game/Player/Weapon/BP_Weapon_Base Object Reference"))
  (return (select `bool` IsAlternative :`false` (`self.CurrentMainWeapon`) :`true` (`self.CurrentAltWeapon`))))

(fn `GetWeaponPoint`
  (params (IsAlternative :type Boolean))
  (returns (WeaponPoint :type "SceneComponent Object Reference"))
  (return (select `bool` IsAlternative :`false` (`self.MainWeaponPoint`) :`true` (`self.AltWeaponPoint`))))

(fn `GetWeaponsArray`
  (params (IsAlternative :type Boolean))
  (returns (Weapons :type "Array of /Game/Player/Items/BP_Item_Base Object Reference"))
  (return (select `bool` IsAlternative :`false` (`self.MainWeapons`) :`true` (`self.AlternativeWeapons`))))

(fn `UserConstructionScript`)